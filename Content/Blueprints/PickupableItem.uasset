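; PickupableItem is a world item actor that can be picked up, dropped and thrown.
; The construction script fills its item struct from a data table row keyed by the per-instance item ID, labels a TextRender with the display name and caches the mesh scale.
; Pickup hides and zero-scales the mesh instead of destroying it, and drop restores both.
; Throwing applies a velocity-change impulse along the root's forward vector.
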(event `ItemPickedUp`
  (`SceneComponent.SetVisibility` (`self.ItemMesh`) false true)
  (`SceneComponent.SetWorldScale3D` (`self.ItemMesh`) (0.0 0.0 0.0)))

(event `ItemDropped`
  (`SceneComponent.SetVisibility` (`self.ItemMesh`) true true)
  (`SceneComponent.SetWorldScale3D` (`self.ItemMesh`) (`self.StartScale`)))

(event `ThrowItem`
  (`PrimitiveComponent.AddImpulse` (`self.ItemMesh`) (* (`SceneComponent.GetForwardVector` (`self.DefaultSceneRoot`)) 500.0) "None" true))

(fn `UserConstructionScript`
  (`|ExecutionSequence`
    (:`then_0`
      (bind _returnvalue (`|GetDataTableRow` "/Game/Blueprints/ItemData.ItemData" (`KismetStringLibrary.Conv_StringToName` (`KismetStringLibrary.Conv_IntToString` (`self.ItemID_SETTHIS`))))
        (:`then`
          (bind (_itemid _itemdisplayname _maxdurability _interactmode) (break `/Game/Blueprints/ItemDataStruct` _returnvalue))
          (set `self.ItemData` (make `/Game/Blueprints/ItemDataStruct` _itemid _itemdisplayname _maxdurability _interactmode)))))
    (:`then_1`
      (`TextRenderComponent.K2_SetText` (`self.TextRender`) (`.ItemDisplayName_3_0D7FC95D4783C3BCF9016BBCB2149AFF` (break `/Game/Blueprints/ItemDataStruct` (`self.ItemData`)))))
    (:`then_2`
      (set `self.StartScale` (`SceneComponent.K2_GetComponentScale` (`self.ItemMesh`))))))