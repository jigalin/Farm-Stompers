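; Farm tile actor that runs a shovel, seed, water, grow and harvest cycle through an integer STATE.
; SeedTile loads seed data from the PlantData table; WaterTile starts a timeline scaling the plant's height until harvestable.
; ShovelFunc tills empty soil or harvests, returning a placeholder score instead of the seed's ScoreAdded.
; HighlightTile flashes green or red by tool-state match, while actions swap materials and Niagara splash effects.
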(event `HighlightTile`
  (params (Tool :type Integer))
  ;[1 1 1] HighLight logic
  (if (== Tool (`self.STATE`))
    (`PrimitiveComponent.SetMaterial` (`self.PlaneBG`) 0 "/Game/ArtAssets/Materials/TileHighlightGreen.TileHighlightGreen")
    (`SceneComponent.SetVisibility` (`self.PlaneBG`) true false)
    (`KismetSystemLibrary.RetriggerableDelay` 0.02)
    (`SceneComponent.SetVisibility` (`self.PlaneBG`) false false)
    (else
      (`PrimitiveComponent.SetMaterial` (`self.PlaneBG`) 0 "/Game/ArtAssets/Materials/TileHighlightRed.TileHighlightRed")
      (`SceneComponent.SetVisibility` (`self.PlaneBG`) true false)
      (`KismetSystemLibrary.RetriggerableDelay` 0.02)
      (`SceneComponent.SetVisibility` (`self.PlaneBG`) false false))))

(event `Seed Tile`
  (params (SeedRefInt :type Integer))
  (bind _niagara (`self.Niagara`))
  (bind _plant (`self.Plant`))
  (bind _returnvalue (`|GetDataTableRow` "/Game/Blueprints/PlantData.PlantData" (`KismetStringLibrary.Conv_StringToName` (`KismetStringLibrary.Conv_IntToString` SeedRefInt)))
    (:`then`
      (bind (_seedindex _plantname _specialseedindex _scoreadded _timeinseconds) (break `/Game/Blueprints/PlantStruct` _returnvalue))
      (set `self.SeedVariable` (make `/Game/Blueprints/PlantStruct` _seedindex _plantname _specialseedindex _scoreadded _timeinseconds))
      (if (== (`self.STATE`) 1)
        (`SceneComponent.SetWorldScale3D` _plant (`KismetMathLibrary.MakeVector` (.x (`SceneComponent.K2_GetComponentScale` _plant)) (.y (`SceneComponent.K2_GetComponentScale` _plant)) 0.1))
        (set `self.STATE` 2)
        (`NiagaraComponent.SetAsset` _niagara "/Game/ArtAssets/Particles/SplashGreenSys.SplashGreenSys")
        (`ActorComponent.Activate` _niagara false)))))

(event `Water Tile`
  (bind _plant (`self.Plant`))
  (if (== (`self.STATE`) 2)
    (`NiagaraComponent.SetAsset` (`self.Niagara`) "/Game/ArtAssets/Particles/SplashBlue_System.SplashBlue_System")
    (`PrimitiveComponent.SetMaterial` (`self.Plane`) 0 "/Game/ArtAssets/Materials/Temp_WateredMat.Temp_WateredMat")
    (set `self.STATE` 99)
    ;[1 0 0] Comment
    (bind (_direction _newtrack_0) (`Timeline|Grow` :!via `PlayFromStart`)
      (:`Update`
        (`SceneComponent.SetWorldScale3D` _plant (`KismetMathLibrary.MakeVector` (.x (`SceneComponent.K2_GetComponentScale` _plant)) (.y (`SceneComponent.K2_GetComponentScale` _plant)) _newtrack_0)))
      (:`Finished`
        (set `self.STATE` 0)
        (`PrimitiveComponent.SetMaterial` (`self.Plane`) 0 "/Game/StarterContent/Materials/M_Basic_Wall.M_Basic_Wall")
        (set `self.HasPlant` true)))))

(fn `ShovelFunc`
  (returns (Score :type "Float (double-precision)") (GotPlant :type Boolean))
  (bind _niagara (`self.Niagara`))
  (bind _plant (`self.Plant`))
  (bind _niagara_2 (`self.Niagara`))
  (if (== (`self.STATE`) 0)
    (if (`self.HasPlant`)
      (`SceneComponent.SetWorldScale3D` _plant (`KismetMathLibrary.MakeVector` (.x (`SceneComponent.K2_GetComponentScale` _plant)) (.y (`SceneComponent.K2_GetComponentScale` _plant)) 0.0))
      (`PrimitiveComponent.SetMaterial` (`self.Plane`) 0 "/Game/StarterContent/Materials/M_Basic_Wall.M_Basic_Wall")
      (set `self.STATE` 0)
      (set `self.HasPlant` false)
      (`NiagaraComponent.SetAsset` _niagara "/Game/ArtAssets/Particles/SplashBrown_System.SplashBrown_System")
      (`ActorComponent.Activate` _niagara false)
      (return (`self.PlantScore TEMP`) true)
      (else
        (`PrimitiveComponent.SetMaterial` (`self.Plane`) 0 "/Game/ArtAssets/Materials/Temp_ShovelledMat.Temp_ShovelledMat")
        (set `self.STATE` 1)
        (`NiagaraComponent.SetAsset` _niagara_2 "/Game/ArtAssets/Particles/SplashBrown_System.SplashBrown_System")
        (`ActorComponent.Activate` _niagara_2 false)
        (return 0.0 false)))))

(fn `UserConstructionScript`)