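; FS_Gamemode_1 is a game mode Blueprint that sets up local multiplayer characters at BeginPlay.
; It gathers every PlayerStart, then matches each one's tag to a player index below MaxPlayerCount.
; For each match it creates a local player, spawns a CharacterBP at that start and has that player's controller possess it.
; Each character receives the index as its PlayerQuadrant and is added to the Players array.
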(event `self.ReceiveBeginPlay`
  (`self.GetPlayerStartPoints`)
  (`self.SpawnPlayers`))

(fn `GetPlayerStartPoints`
  (bind _outactors (`GameplayStatics.GetAllActorsOfClass` "/Script/Engine.PlayerStart"))
  (set `self.PlayerStarts` _outactors))

(fn `SpawnPlayers`
  (for _index (range (`self.MaxPlayerCount`))
    (set `self.Index` _index)
    (for _array_element (`self.PlayerStarts`)
      (if (== (`PlayerStart.PlayerStartTag` _array_element) (`KismetStringLibrary.Conv_IntToString` (`self.Index`)))
        (`GameplayStatics.CreatePlayer` (`self.Index`))
        (bind _returnvalue (`|SpawnActorFromClass` "/Game/Blueprints/CharacterBP.CharacterBP_C" (`self.GetTransform` _array_element) "AlwaysSpawn" "OverrideRootScale" null null))
        (`Controller.Possess` (`GameplayStatics.GetPlayerController` (`self.Index`)) _returnvalue)
        (set `/Game/Blueprints/CharacterBP.PlayerQuadrant` (`self.Index`) _returnvalue)
        (`KismetArrayLibrary.Array_AddUnique` (`self.Players`) _returnvalue)))))

(fn `UserConstructionScript`)